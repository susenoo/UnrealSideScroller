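; A 2D platform lift that moves its grass platform sprite between its origin and EndLocation.
; The AnimationLift timeline lerps the position at a rate derived from TravelTimeInSeconds, and on finishing waits StopDelay before running the opposite way.
; A Character overlapping the safety collider calls Play or Reverse on the active timeline, depending on whether it is playing.
; The construction script applies LiftColor and previews the end position via TestEndLocation.
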(event OnComponentBeginOverlap(SaftyCollider)
  (params (OverlappedComponent :type Primitive%20Component%20Object%20Reference) (OtherActor :type Actor%20Object%20Reference) (OtherComp :type Primitive%20Component%20Object%20Reference) (OtherBodyIndex :type Integer) (bFromSweep :type Boolean) (SweepResult :type Hit%20Result%20Structure%20%28by%20ref%29))
  (bind _animationlift (Variables|Default|GetanimationLift))
  (Utilities|Casting|CastToCharacter OtherActor)
  (if (Components|Activation|IsActive _animationlift)
    (if (Audio|Components|Audio|IsPlaying _animationlift)
      (bind (_direction _alphalerp) (Timeline|animationLift Play)
        (:Update
          (Transformation|SetRelativeLocation (Variables|Default|GetGrassPlatfomr01_Sprite) (Math|Vector|Lerp(Vector) "0, 0, 0" (Variables|LiftControls|GetEndLocation) _alphalerp) false false))
        (:Finished
          (Utilities|FlowControl|Delay (Variables|LiftControls|GetStopDelay))
          (switch Utilities|FlowControl|Switch|SwitchonETimelineDirection _direction
            (:Forward
              (CallFunction|PlayLiftBackwards))
            (:Backward
              (CallFunction|PlayLiftForward)))))
      (else
        (Timeline|animationLift Reverse)))))

(event Custom|PlayLiftForward
  (bind (_direction _alphalerp) (Timeline|animationLift PlayFromStart)
    (:Update
      (Transformation|SetRelativeLocation (Variables|Default|GetGrassPlatfomr01_Sprite) (Math|Vector|Lerp(Vector) "0, 0, 0" (Variables|LiftControls|GetEndLocation) _alphalerp) false false))
    (:Finished
      (Utilities|FlowControl|Delay (Variables|LiftControls|GetStopDelay))
      (switch Utilities|FlowControl|Switch|SwitchonETimelineDirection _direction
        (:Forward
          (CallFunction|PlayLiftBackwards))
        (:Backward
          (CallFunction|PlayLiftForward))))))

(event Custom|PlayLiftBackwards
  (bind (_direction _alphalerp) (Timeline|animationLift ReverseFromEnd)
    (:Update
      (Transformation|SetRelativeLocation (Variables|Default|GetGrassPlatfomr01_Sprite) (Math|Vector|Lerp(Vector) "0, 0, 0" (Variables|LiftControls|GetEndLocation) _alphalerp) false false))
    (:Finished
      (Utilities|FlowControl|Delay (Variables|LiftControls|GetStopDelay))
      (switch Utilities|FlowControl|Switch|SwitchonETimelineDirection _direction
        (:Forward
          (CallFunction|PlayLiftBackwards))
        (:Backward
          (CallFunction|PlayLiftForward))))))

(event EventBeginPlay
  (Components|Timeline|SetPlayRate (Variables|Default|GetanimationLift) (/ (Variables|LiftControls|GetTravelTimeInSeconds) 1.0))
  (Variables|LiftControls|SetTestEndLocation false))

(fn ConstructionScript
  (Transformation|SetRelativeLocation (Variables|Default|GetGrassPlatfomr01_Sprite) (Math|Vector|SelectVector (Variables|LiftControls|GetEndLocation) "0, 0, 0" (Variables|LiftControls|GetTestEndLocation)) false false)
  (Sprite|SetSpriteColor (Variables|Default|GetGrassPlatfomr01_Sprite) (Variables|LiftControls|GetLiftColor)))